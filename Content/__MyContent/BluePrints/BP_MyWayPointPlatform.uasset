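; Moving platform that travels through an ordered array of waypoint actors, with a configurable mesh and material applied at construction.
; BeginPlay hides the waypoints and starts a rate-scaled timeline, intended to lerp the platform between the current and next waypoint positions.
; The timeline's event track advances the waypoint indices and replays, or restarts from the first waypoint when Loop is set.
; Start and Stop functions control the motion.
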(event `self.ReceiveBeginPlay`
  (for _array_element (`self.waypoints`)
    (`self.SetActorHiddenInGame` _array_element true)
    (`self.platform start`)))

(event `platform start`
  (bind _motion_timeline (`self.motion timeline`))
  (`self.set first waypoint`)
  (`TimelineComponent.SetPlayRate` _motion_timeline (`self.rate`))
  (`TimelineComponent.PlayFromStart` _motion_timeline))

(fn `path is finished`
  (returns (`path finished` :type Boolean))
  (return (== (`self.next waypoint index`) (- (`KismetArrayLibrary.Array_Length` (`self.waypoints`)) 1))))

(fn `set first waypoint`
  (set `self.current waypoint index` 0)
  (set `self.next waypoint index` 1)
  (`self.set positions`))

(fn `set next waypoint`
  (bind _result (`/Engine/EditorBlueprintResources/StandardMacros.IncrementInt` (`self.current waypoint index`))
    (:`  `
      (set `self.next waypoint index` (+ _result 1))
      (`self.set positions`))))

(fn `set positions`
  (bind _waypoints (`self.waypoints`))
  (set `self.current waypoint position` (`self.K2_GetActorLocation` (`|GetArrayItem` _waypoints (`self.current waypoint index`))))
  (set `self.next way position` (`self.K2_GetActorLocation` (`|GetArrayItem` _waypoints (`self.next waypoint index`)))))

(fn `start`
  (`self.platform start`))

(fn `stop`
  (`TimelineComponent.Stop` (`self.motion timeline`)))

(fn `UserConstructionScript`
  (bind _platofrm_mesh (`self.platofrm Mesh`))
  (`StaticMeshComponent.SetStaticMesh` _platofrm_mesh (`self.static mesh`))
  (`PrimitiveComponent.SetMaterial` _platofrm_mesh 0 (`self.static material`)))