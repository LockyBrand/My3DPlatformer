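; Game mode that locates the game manager actor and provides setup for the game's UI.
; BeginPlay caches the first BP_MyGameManager found in the world.
; CreateUI, not called within this graph, creates the options/abandon, win, lose and health bar widgets, stores each on the manager returned by GetGameManager, and adds all to the viewport immediately.
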(event `self.ReceiveBeginPlay`
  (bind _outactors (`GameplayStatics.GetAllActorsOfClass` "/Game/__MyContent/BluePrints/BP_MyGameManager.BP_MyGameManager_C"))
  (set `self.manager` (`|GetArrayItem` _outactors)))

(fn `create UI`
  (bind _mygamemanager (`/Game/__MyContent/BluePrints/BP_MyFunctionLibrary.get game manager`))
  (bind _returnvalue (`|CreateWidget` "/Game/__MyContent/widgets/MyOptions.MyOptions_C"))
  (bind _output_get (set `/Game/__MyContent/BluePrints/BP_MyGameManager.widget_abandon` _returnvalue _mygamemanager))
  (`UserWidget.AddToViewport` _output_get 0)
  (bind _returnvalue_2 (`|CreateWidget` "/Game/__MyContent/widgets/widget_WIN.widget_WIN_C"))
  (bind _output_get_2 (set `/Game/__MyContent/BluePrints/BP_MyGameManager.widget_WIN` _returnvalue_2 _mygamemanager))
  (`UserWidget.AddToViewport` _output_get_2 0)
  (bind _returnvalue_3 (`|CreateWidget` "/Game/__MyContent/widgets/widget_LOSE.widget_LOSE_C"))
  (bind _output_get_3 (set `/Game/__MyContent/BluePrints/BP_MyGameManager.widget_LOSE` _returnvalue_3 _mygamemanager))
  (`UserWidget.AddToViewport` _output_get_3 0)
  (bind _returnvalue_4 (`|CreateWidget` "/Game/__MyContent/widgets/widget_helth.widget_helth_C"))
  (bind _output_get_4 (set `/Game/__MyContent/BluePrints/BP_MyGameManager.widget_HealthBar` _returnvalue_4 _mygamemanager))
  (`UserWidget.AddToViewport` _output_get_4 0))

(fn `UserConstructionScript`)