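; BP_mySplinePlatform is a platform actor that moves its mesh along a spline, starting at BeginPlay.
; A timeline, played at a speed set by Rate, outputs a SplineDistance fraction that is scaled by spline length to set the mesh's world location without sweeping.
; The construction script applies the StaticMesh and Material variables to the platform mesh.
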(event `self.ReceiveBeginPlay`
  (`self.platform start`))

(event `platform start`
  (bind _spline (`self.Spline`))
  (`TimelineComponent.SetPlayRate` (`self.motion timeline`) (`self.rate`))
  (bind (_direction _spline_distance) (`Timeline|motion timeline` :!via `PlayFromStart`)
    (:`Update`
      (`SceneComponent.K2_SetWorldLocation` (`self.Platform Mesh`) (`SplineComponent.GetLocationAtDistanceAlongSpline` _spline (* _spline_distance (`SplineComponent.GetSplineLength` _spline)) "World") false false))))

(fn `UserConstructionScript`
  (`StaticMeshComponent.SetStaticMesh` (`self.Platform Mesh`) (`self.Static Mesh`))
  (`PrimitiveComponent.SetMaterial` (`self.Platform Mesh`) 0 (`self.Material`)))